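; UpPressed is an actor that handles the upmap input action for an up arrow, apparently in a rhythm-style game.
; It enables player input on BeginPlay and again every Tick.
; A press spawns an UpHitbox at the Arrow component, then after a brief delay spawns top and bottom boxes at Arrowtop and Arrowbot.
; It then passes Score to the Gamemode through AddTartgetPoint.
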(event `self.ReceiveTick`
  (params (DeltaSeconds :type "Float (single-precision)"))
  (`self.EnableInput` (`GameplayStatics.GetPlayerController` 0)))

(event `self.ReceiveBeginPlay`
  (`self.EnableInput` (`GameplayStatics.GetPlayerController` 0)))

(event `InputAction|upmap`
  (params (Key :type "Key Structure"))
  (:`Pressed`
    (`|SpawnActorFromClass` "/Game/Blueprints/UpArrow/UpHitbox.UpHitbox_C" (`SceneComponent.K2_GetComponentToWorld` (`self.Arrow`)) "Undefined" "OverrideRootScale" null null)
    (`KismetSystemLibrary.Delay` 0.06)
    (`|SpawnActorFromClass` "/Game/Blueprints/UpArrow/UpTopBox.UpTopBox_C" (`SceneComponent.K2_GetComponentToWorld` (`self.arrowtop`)) "Undefined" "OverrideRootScale" null null)
    (`|SpawnActorFromClass` "/Game/Blueprints/UpArrow/UpBotBox.UpBotBox_C" (`SceneComponent.K2_GetComponentToWorld` (`self.arrowbot`)) "Undefined" "OverrideRootScale" null null)
    (bind _asgamemode (cast `/Game/Blueprints/Gamemode` (`GameplayStatics.GetGameMode`)))
    (`/Game/Blueprints/Gamemode.AddTartgetPoint` _asgamemode (`self.Score`))))

(fn `UserConstructionScript`)