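; LeftPressed1 is a left-arrow input actor that spawns hitboxes when the leftmap action is pressed.
; It enables player 0 input on BeginPlay and again every Tick.
; Each press spawns LeftHitbox at Arrow, then after a brief delay spawns LeftTopBox and LeftBotbox at the top and bottom arrow components.
; It then passes Score to the Gamemode's AddTartgetPoint on every press, with no hit check in this graph.
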(event `self.ReceiveTick`
  (params (DeltaSeconds :type "Float (single-precision)"))
  (`self.EnableInput` (`GameplayStatics.GetPlayerController` 0)))

(event `self.ReceiveBeginPlay`
  (`self.EnableInput` (`GameplayStatics.GetPlayerController` 0)))

(event `InputAction|leftmap`
  (params (Key :type "Key Structure"))
  (:`Pressed`
    (`|SpawnActorFromClass` "/Game/Blueprints/LeftArrow/LeftHitbox.LeftHitbox_C" (`SceneComponent.K2_GetComponentToWorld` (`self.Arrow`)) "Undefined" "OverrideRootScale" null null)
    (`KismetSystemLibrary.Delay` 0.06)
    (`|SpawnActorFromClass` "/Game/Blueprints/LeftArrow/LeftTopBox.LeftTopBox_C" (`SceneComponent.K2_GetComponentToWorld` (`self.arrowtop`)) "Undefined" "OverrideRootScale" null null)
    (`|SpawnActorFromClass` "/Game/Blueprints/LeftArrow/LeftBotbox.LeftBotbox_C" (`SceneComponent.K2_GetComponentToWorld` (`self.arrowbot`)) "Undefined" "OverrideRootScale" null null)
    (bind _asgamemode (cast `/Game/Blueprints/Gamemode` (`GameplayStatics.GetGameMode`)))
    (`/Game/Blueprints/Gamemode.AddTartgetPoint` _asgamemode (`self.Score`))))

(fn `UserConstructionScript`)