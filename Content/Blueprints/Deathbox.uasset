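; Deathbox is a trigger actor that destroys any actor overlapping it and reports score and lives to the Gamemode.
; Actor overlap destroys the other actor, then passes Score to the Gamemode's AddTartgetPoint.
; A separate Box component overlap passes Lives to LivesPoint without filtering what entered.
; On BeginPlay it also creates the BP_Hud widget and adds it to the viewport.
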(event `self.ReceiveBeginPlay`
  (bind _returnvalue (`|CreateWidget` "/Game/Blueprints/BP_Hud.BP_Hud_C"))
  (`UserWidget.AddToViewport` _returnvalue 0))

(event `self.ReceiveActorBeginOverlap`
  (params (OtherActor :type "Actor Object Reference"))
  (`self.K2_DestroyActor` OtherActor)
  (bind _asgamemode (cast `/Game/Blueprints/Gamemode` (`GameplayStatics.GetGameMode`)))
  (`/Game/Blueprints/Gamemode.AddTartgetPoint` _asgamemode (`self.Score`)))

(event `self.Box.OnComponentBeginOverlap`
  (params (OverlappedComponent :type "PrimitiveComponent Object Reference") (OtherActor :type "Actor Object Reference") (OtherComp :type "PrimitiveComponent Object Reference") (OtherBodyIndex :type Integer) (bFromSweep :type Boolean) (SweepResult :type "HitResult Structure (by ref)"))
  (bind _asgamemode (cast `/Game/Blueprints/Gamemode` (`GameplayStatics.GetGameMode`)))
  (`/Game/Blueprints/Gamemode.LivesPoint` _asgamemode (`self.Lives`)))

(fn `UserConstructionScript`)