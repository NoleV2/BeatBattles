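; Game mode Blueprint that tracks the player's score and lives for the game.
; Custom events subtract from Lives and add target points to Score.
; Tick compares Lives against Lifebase every frame and opens the ES_Game level by name once Lives falls below it.
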(event `self.ReceiveTick`
  (params (DeltaSeconds :type "Float (single-precision)"))
  (if (< (`self.Lives`) (`self.lifebase`))
    (`GameplayStatics.OpenLevel` "ES_Game")))

(event `LivesPoint`
  (params (`Remove Lives` :type Integer))
  (set `self.Lives` (- (`self.Lives`) `Remove Lives`)))

(event `AddTartgetPoint`
  (params (AddScore :type Integer))
  (set `self.Score` (+ AddScore (`self.Score`))))

(fn `UserConstructionScript`)