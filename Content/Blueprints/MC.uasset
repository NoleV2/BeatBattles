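; MC is a Blueprint that switches the MC flipbook between four dance animations, one per direction event.
; LeftP, DownP, UpP and RightP each set their own MCDANCE flipbook, wait one second, set IdleC and call IdleSwitch.
; IdleSwitch only tests IdleC and does nothing after the branch, so no return to an idle animation happens here.
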(event `LeftP`
  (`PaperFlipbookComponent.SetFlipbook` (`self.MC`) "/Game/Sprites/MCDANCE4.MCDANCE4")
  (`KismetSystemLibrary.Delay` 1.0)
  (set `self.IdleC` true)
  (`self.IdleSwitch`))

(event `DownP`
  (`PaperFlipbookComponent.SetFlipbook` (`self.MC`) "/Game/Sprites/MCDANCE3.MCDANCE3")
  (`KismetSystemLibrary.Delay` 1.0)
  (set `self.IdleC` true)
  (`self.IdleSwitch`))

(event `UpP`
  (`PaperFlipbookComponent.SetFlipbook` (`self.MC`) "/Game/Sprites/MCDANCE2.MCDANCE2")
  (`KismetSystemLibrary.Delay` 1.0)
  (set `self.IdleC` true)
  (`self.IdleSwitch`))

(event `RightP`
  (`PaperFlipbookComponent.SetFlipbook` (`self.MC`) "/Game/Sprites/MCDANCE1.MCDANCE1")
  (`KismetSystemLibrary.Delay` 1.0)
  (set `self.IdleC` true)
  (`self.IdleSwitch`))

(event `IdleSwitch`
  (if (`self.IdleC`)
    _))

(fn `UserConstructionScript`)